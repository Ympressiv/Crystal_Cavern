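; BP_Crystal is a collectible that flies to the player on overlap, enlarges them and awards points.
; It stores its location, scale and light intensity, then a timeline lerps it toward the player's current position.
; When that finishes, it shrinks and dims in one step using the timeline's final values.
; A second timeline grows the player in X and Y from their current scale each update, then calls Points and destroys the crystal.
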(event `self.ReceiveActorBeginOverlap`
  (params (OtherActor :type "Actor Object Reference"))
  (`/Game/Actors/Libraries/MacroLibrary.IsPlayer` OtherActor
    (:`IsPlayer`
      (`self.Store Starting Values`)
      (bind (_direction _smooth_lerp_alpha _scale_progress _light_intensity) (`Timeline|Alpha Blend Timeline`)
        (:`Update`
          (bind _returnvalue (`self.MoveToPlayer` _smooth_lerp_alpha)))
        (:`Finished`
          (bind _asbp_player_pawn (cast `/Game/Actors/Pawn/BP_PlayerPawn` _returnvalue))
          (`self.ScaleMinusCrystal` _scale_progress)
          (`self.LightCrystal` _light_intensity)
          (bind (_direction_2 _smooth_lerp_alpha_2) (`Timeline|ScaleTime`)
            (:`Update`
              (`self.ScaleUp` _smooth_lerp_alpha_2))
            (:`Finished`
              (`/Game/Actors/Pawn/BP_PlayerPawn.Points` _asbp_player_pawn)
              (`self.K2_DestroyActor`))))))))

(fn `LightCrystal`
  (params (Alpha :type "Float (double-precision)"))
  (`LightComponent.SetIntensity` (`self.PointLight`) (`KismetMathLibrary.Lerp` (`self.Intensity`) 0.0 Alpha)))

(fn `MoveToPlayer`
  (params (Alpha :type "Float (double-precision)"))
  (returns (ReturnValue :type "Pawn Object Reference"))
  (bind _returnvalue (`GameplayStatics.GetPlayerPawn` 0))
  (`self.K2_SetActorLocation` (`KismetMathLibrary.VLerp` (`self.Lerp Start Location`) (`self.K2_GetActorLocation` _returnvalue) Alpha))
  (return _returnvalue))

(fn `ScaleMinusCrystal`
  (params (Alpha :type "Float (double-precision)"))
  (`self.SetActorScale3D` (`KismetMathLibrary.VLerp` (`self.ScaleCrystal`) (0.0 0.0 0.0) Alpha)))

(fn `ScaleUp`
  (params (Alpha :type "Float (double-precision)"))
  (bind _returnvalue (`GameplayStatics.GetPlayerPawn` 0))
  (bind _returnvalue_2 (`self.GetActorScale3D` _returnvalue))
  (`self.SetActorScale3D` _returnvalue (`KismetMathLibrary.VLerp` _returnvalue_2 (+ _returnvalue_2 (0.25 0.25 0.0)) Alpha)))

(fn `Store Starting Values`
  (set `self.Lerp Start Location` (`self.K2_GetActorLocation`))
  (set `self.ScaleCrystal` (`self.GetActorScale3D`))
  (set `self.Intensity` (`LightComponentBase.Intensity` (`self.PointLight`))))

(fn `UserConstructionScript`)