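; Cannon actor that automatically fires projectiles on an endless loop from BeginPlay.
; Each cycle waits FireRate, then spawns a BO_Projectitles at the ProjectileSpawn component's location and rotation, scaled by ProjectitlesScale.
; The Cannon_Fire timeline then animates the barrel's relative location, and its Finished output restarts the delay, so the shot interval is the delay plus the timeline length.
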(event `self.ReceiveBeginPlay`
  (`KismetSystemLibrary.Delay` (`self.FireRate`) :!label _label)
  (`self.SpawnProjectitle`)
  (bind (_direction _cannon_location) (`Timeline|Cannon_Fire` :!via `PlayFromStart`)
    (:`Update`
      (`self.MoveCanon` _cannon_location))
    (:`Finished`
      (goto _label))))

(fn `MoveCanon`
  (params (NewLocation_Y :type "Float (double-precision)"))
  (`SceneComponent.K2_SetRelativeLocation` (`self.Cannon Barrel`) (`KismetMathLibrary.MakeVector` 0.0 NewLocation_Y) false false))

(fn `SpawnProjectitle`
  (bind _projectile_spawn (`self.Projectile Spawn`))
  (`|SpawnActorFromClass` "/Game/Actors/Projectitles_Shot/BO_Projectitles.BO_Projectitles_C" (`KismetMathLibrary.MakeTransform` (`SceneComponent.K2_GetComponentLocation` _projectile_spawn) (`SceneComponent.K2_GetComponentRotation` _projectile_spawn) (`KismetMathLibrary.Conv_DoubleToVector` (`self.Projectitles_Scale`))) "Undefined" "OverrideRootScale" null null))

(fn `UserConstructionScript`)