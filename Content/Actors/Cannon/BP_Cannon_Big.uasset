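; BP_Cannon_Big is a cannon actor that automatically fires big projectiles on a repeating timer from BeginPlay.
; Each cycle waits for FireRate, then spawns a BO_Projectitles_Big at the ProjectileSpawn component's location and rotation, scaled by ProjectitlesScale.
; A timeline then animates the Cannon component's relative Y position, likely as recoil, and its Finished output loops back to the delay.
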(event `self.ReceiveBeginPlay`
  (`KismetSystemLibrary.Delay` (`self.FireRate`) :!label _label)
  (`self.NewFunction_0`)
  (bind (_direction _cannon_location) (`Timeline|Timeline_0` :!via `PlayFromStart`)
    (:`Update`
      (`self.NewFunction_1` _cannon_location))
    (:`Finished`
      (goto _label))))

(fn `NewFunction_0`
  (bind _projectile_spawn (`self.Projectile Spawn`))
  (`|SpawnActorFromClass` "/Game/Actors/Projectitles_Shot/BO_Projectitles_Big.BO_Projectitles_Big_C" (`KismetMathLibrary.MakeTransform` (`SceneComponent.K2_GetComponentLocation` _projectile_spawn) (`SceneComponent.K2_GetComponentRotation` _projectile_spawn) (`KismetMathLibrary.Conv_DoubleToVector` (`self.Projectitles_Scale`))) "Undefined" "OverrideRootScale" null null))

(fn `NewFunction_1`
  (params (NewLocation_Y :type "Float (double-precision)"))
  (`SceneComponent.K2_SetRelativeLocation` (`self.Cannon`) (`KismetMathLibrary.MakeVector` 0.0 NewLocation_Y) false false))

(fn `UserConstructionScript`)