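; BP_PlayerPawn is the player pawn, a physics-driven mesh moved by torque from the movement axes, scaled by Acceleration.
; Any damage or a Reset event runs a one-shot restart macro that shows a death message, fades out and reloads the level.
; It also fades in on start, counts and prints crystal points, and quits on Escape.
; AdjustCameraChange sets the spring arm's length and rotation.
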(event `InputAxis|Move Right/Left`
  (params (AxisValue :type "Float (single-precision)"))
  (bind (_mesh _returnvalue _returnvalue2) (`self.WASD` AxisValue (stale `InputAxis|Move Forwards/Backwards` AxisValue) :!label _label))
  (`PrimitiveComponent.AddTorqueInRadians` _mesh (`KismetMathLibrary.MakeVector` _returnvalue) "None" true)
  (`PrimitiveComponent.AddTorqueInRadians` _mesh (`KismetMathLibrary.MakeVector` 0.0 _returnvalue2) "None" true))

(event `InputAxis|Move Forwards/Backwards`
  (params (AxisValue :type "Float (single-precision)"))
  (goto _label))

(event `Key|Escape`
  (params (Key :type "Key Structure"))
  (:`Pressed`
    (`KismetSystemLibrary.QuitGame` null "Quit")))

(event `self.ReceiveAnyDamage`
  (params (Damage :type "Float (single-precision)") (DamageType :type "DamageType Object Reference") (InstigatedBy :type "Controller Object Reference") (DamageCauser :type "Actor Object Reference"))
  ;[1 1 1] Reset
  (`self.Restart Level` :!label _label_2))

(event `self.ReceiveBeginPlay`
  ;[1 1 1] FADE IN
  (`PlayerCameraManager.StartCameraFade` :`self` (`GameplayStatics.GetPlayerCameraManager` 0) :`FromAlpha` 1.0 :`Duration` 5.0))

(event `Points`
  ;[1 1 1] POINTS
  (bind _result (`/Engine/EditorBlueprintResources/StandardMacros.IncrementInt` (`self.Point`))
    (:`  `
      (`KismetSystemLibrary.PrintString` (`KismetStringLibrary.Concat_StrStr` "Crystal points: " (`KismetStringLibrary.Conv_IntToString` _result)) true true (struct :`R` 0.701675 :`G` 0.71875 :`A` 1.0) 3.0))))

(event `Reset`
  ;[1 1 1] Reset
  (goto _label_2))

(fn `AdjustCameraChange`
  (params (Distance :type "Float (double-precision)") (PitchZ :type "Float (double-precision)") (PitchY :type "Float (double-precision)"))
  (bind _springarm (`self.SpringArm`))
  (set `SpringArmComponent.TargetArmLength` Distance _springarm)
  (`SceneComponent.K2_SetWorldRotation` _springarm (`KismetMathLibrary.MakeRotator` 0.0 PitchY PitchZ) false false))

(fn `UserConstructionScript`)

(fn `WASD`
  (params (A :type "Float (double-precision)") (A2 :type "Float (double-precision)"))
  (returns (Mesh :type "StaticMeshComponent Object Reference") (ReturnValue :type "Float (double-precision)") (ReturnValue2 :type "Float (double-precision)"))
  (bind _acceleration (`self.Acceleration`))
  (return (`self.Mesh`) (* A _acceleration) (* A2 _acceleration)))